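; BP_MenuCamera is a camera actor that moves continuously along a spline, apparently as a menu backdrop.
; On BeginPlay it becomes the first player controller's view target with a short blend and moves the player pawn to a fixed point above the world origin.
; Each tick it advances a time value, wraps it by the spline's duration, and places the camera at that constant-velocity spline transform, producing a looping flythrough.
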(event EventBeginPlay
  (Game|Player|SetViewTargetwithBlend (Game|GetPlayerController 0) self 0.1 "VTBlend_Linear" 0.0 false)
  (Transformation|SetActorLocation (Game|Player|GetPlayerPawn 0) "0, 0,1000.000000" false false))

(event EventTick
  (params (DeltaSeconds :type Float%20%28single-precision%29))
  (bind _spline (Variables|Default|GetSpline))
  (bind _output_get (Variables|Default|SetTime (Math|Float|%(Float) (+ (Variables|Default|GetTime) DeltaSeconds) (Variables|/Script/Engine.SplineComponent|GetDuration _spline))))
  (Transformation|SetWorldTransform (Variables|Default|GetCamera) (Spline|GetTransformatTime _spline _output_get "World" true true) false false))

(fn ConstructionScript)