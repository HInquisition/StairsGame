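; Player controller for the menu that creates the menu widgets and switches which one is visible.
; On BeginPlay it adds the main menu and a collapsed texture settings widget, with events to show or hide each.
; OpenSettings toggles a freshly created settings widget against the main menu, and the widget's close request reuses the closing branch.
; The cursor stays visible in both states, and the input mode switches are disconnected.
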(event Custom|CloseRequested
  (Widget|RemovefromParent (stale Custom|OpenSettings _returnvalue))
  (Variables|Default|SetbShowMouseCursor true)
  (Variables|Default|SetSettingsOpen false)
  (Widget|SetVisibility (Variables|Default|GetMainMenu) "Visible"))

(event Custom|OpenSettings
  (bind _mainmenu (Variables|Default|GetMainMenu))
  (if (Variables|Default|GetSettingsOpen)
    (Widget|RemovefromParent (stale _returnvalue))
    (Variables|Default|SetbShowMouseCursor true)
    (Variables|Default|SetSettingsOpen false)
    (Widget|SetVisibility _mainmenu "Visible")
    (else
      (bind _returnvalue (UserInterface|CreateWidget "/Game/UI/SettingsUI.SettingsUI_C"))
      (EventDispatchers|BindEventtoCloseRequested _returnvalue (delegate Custom|CloseRequested))
      (UserInterface|Viewport|AddtoViewport _returnvalue 0)
      (Variables|Default|SetbShowMouseCursor true)
      (Variables|Default|SetSettingsOpen true)
      (Widget|SetVisibility _mainmenu "Collapsed"))))

(event Custom|SetMainMenuVisibility
  (params (Visible? :type Boolean))
  (Widget|SetVisibility (Variables|Default|GetMainMenu) (select Visible? "Visible" "Collapsed")))

(event Custom|SetTextureMenuVisibility
  (params (Visible? :type Boolean))
  (Widget|SetVisibility (Variables|Default|GetTextureSettings) (select Visible? "Visible" "Collapsed")))

(event EventBeginPlay
  (bind _returnvalue (UserInterface|CreateWidget "/Game/Widgets/WB_MainMenu.WB_MainMenu_C"))
  (Variables|Default|SetMainMenu _returnvalue)
  (UserInterface|Viewport|AddtoViewport _returnvalue 0)
  (bind _returnvalue_2 (UserInterface|CreateWidget "/Game/ImportTexture/WB_TExtureSettings.WB_TextureSettings_C"))
  (bind _output_get (Variables|Default|SetTextureSettings _returnvalue_2))
  (UserInterface|Viewport|AddtoViewport _output_get 0)
  (Widget|SetVisibility _output_get "Collapsed"))

(fn ConstructionScript)