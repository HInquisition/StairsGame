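; BP_Text is an actor that displays text in the world through a WB_Text widget on its Widget component.
; A shared function pushes the actor's Font, Text and ColorAndOpacity into the widget at construction and BeginPlay, and SetText changes the text separately.
; The construction script also calls the widget's Update and nudges the actor slightly along world Y on every run; its Refresh-flag branch is unconnected.
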(event EventBeginPlay
  (CallFunction|NewFunction0))

(event Collision|EventActorBeginOverlap
  (params (OtherActor :type Actor%20Object%20Reference)))

(event EventTick
  (params (DeltaSeconds :type Float%20%28single-precision%29)))

(fn ConstructionScript
  (bind _aswb_text (Utilities|Casting|CastToWB_Text (UserInterface|GetWidget (Variables|Default|GetWidget))))
  (bind _output_get (Variables|Default|SetAs%20WB%20Text _aswb_text))
  (CallFunction|NewFunction0)
  (Default|Update _output_get)
  (Transformation|AddActorWorldOffset "0,0.100000, 0"))

(fn SetText
  (params (NewParam :type Text))
  (bind _aswb_text (Utilities|Casting|CastToWB_Text (UserInterface|GetWidget (Variables|Default|GetWidget))))
  (Default|SetText _aswb_text NewParam))

(fn NewFunction0
  (bind _aswb_text (Utilities|Casting|CastToWB_Text (UserInterface|GetWidget (Variables|Default|GetWidget))))
  (Default|SetFont _aswb_text (Variables|Default|GetFont))
  (Default|SetText _aswb_text (Variables|Default|GetText))
  (Default|SetColor _aswb_text (Variables|Default|GetColor%20and%20Opacity)))