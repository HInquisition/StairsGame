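; BP_SavePoint is an interactable crystal save point that enables respawning for the player who activates it.
; Interact sets the player's CanRespawn flag and changes the text returned by GetHintText to confirm activation.
; It also runs timelines that animate the crystal material's Offset and the mesh's height, alongside a sound and a brief camera shake.
; Once activated, the crystal rotates continuously on Tick.
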(event EventBeginPlay
  (bind _returnvalue (Rendering|Material|CreateDynamicMaterialInstance (Variables|Default|GetStaticMesh) 0 "/Game/Materials/CrystallShader_Inst.CrystallShader_Inst" "None" :!class /Script/Engine.PrimitiveComponent))
  (Variables|Default|SetCrystalMat _returnvalue))

(event Collision|EventActorBeginOverlap
  (params (OtherActor :type Actor%20Object%20Reference)))

(event EventTick
  (params (DeltaSeconds :type Float%20%28single-precision%29))
  (if (Variables|Default|GetIsRotating?)
    (Transformation|AddWorldRotation (Variables|Default|GetStaticMesh) "0.010000,1.000000,0.010000" false false)))

(event EventInteract
  (params (Player :type BP%20Player%20Character%20Object%20Reference))
  (bind _returnvalue (Game|GetPlayerController 0))
  (bind _staticmesh (Variables|Default|GetStaticMesh))
  (bind _relativelocation (Variables|/Script/Engine.SceneComponent|GetRelativeLocation _staticmesh))
  (Variables|/Game/BP/BP_PlayerCharacter.BP_PlayerCharacter_C|SetCanRespawn? Player true)
  (Variables|Default|SetText "Respawn Point Activated")
  (Utilities|FlowControl|Sequence
    (:then_0
      (bind _newtrack_0 (Timeline|Timeline Play)
        (:Update
          (Rendering|Material|SetScalarParameterValue (Variables|Default|GetCrystalMat) "Offset" _newtrack_0 :!class /Script/Engine.MaterialInstanceDynamic))))
    (:then_1
      (Game|Feedback|ClientStartCameraShake _returnvalue "/Game/BP/CAmeraShake.CameraShake_C" 1.0 "CameraLocal" "0, 0, 0")
      (bind _newtrack_1 (Timeline|Timeline_0 Play)
        (:Update
          (Transformation|SetRelativeLocation _staticmesh (Math|Vector|MakeVector (.x _relativelocation) (.y _relativelocation) _newtrack_1) false false))))
    (:then_2
      (Variables|Default|SetIsRotating? true)
      (Utilities|FlowControl|Delay 0.5)
      (Game|Feedback|ClientStopCameraShake _returnvalue "/Game/BP/CAmeraShake.CameraShake_C" true))
    (:then_3
      (Audio|PlaySoundatLocation "/Game/Sounds/SC_CrystalFlying.SC_CrystalFlying" (Transformation|GetActorLocation) "0, 0, 0" 1.0 1.0 0.0 0 0 0))))

(fn ConstructionScript)

(fn GetHintText
  (return (Variables|Default|GetText)))