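; BP_Bed is an interactable bed that shows a "Rest" hint and lets the player rest to reduce exhaustion.
; Interact switches off the flashlight, blends the view to the bed and disables input while a timeline drives the player's post-process vignette.
; The timeline's Finished event lowers exhaustion.
; After a fixed delay, input returns, the vignette reverses, the view blends back to the character and the flashlight switches on.
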(event EventBeginPlay)

(event Collision|EventActorBeginOverlap
  (params (OtherActor :type Actor%20Object%20Reference)))

(event EventTick
  (params (DeltaSeconds :type Float%20%28single-precision%29)))

(event EventInteract
  (params (Player :type BP%20Player%20Character%20Object%20Reference))
  (bind _returnvalue (Game|GetPlayerController 0))
  (bind _output_get (Variables|Default|SetPlayer Player))
  (Class|UserTexturesTesterCharacter|SwitchOffFlashlight _output_get)
  (Game|Player|SetViewTargetwithBlend (Game|GetPlayerController 0) self 1.0 "VTBlend_Linear" 0.0 false)
  (Utilities|FlowControl|Sequence
    (:then_0
      (bind _vignette (Timeline|VignetteTimeline Play)
        (:Update
          (bind _structout (Utilities|Struct|SetmembersinPostProcessSettings (Default|GetPostProcessSettings (Variables|Default|GetPlayer)) _vignette))
          (Default|SetPostProcessSettings (Variables|Default|GetPlayer) _structout))
        (:Finished
          (Default|AddExhaustion (Variables|Default|GetPlayer) -1e+02))))
    (:then_1
      (Input|DisableInput (Variables|Default|GetPlayer) (Game|GetPlayerController 0))
      (Utilities|FlowControl|Delay 5.0)
      (Input|EnableInput (Variables|Default|GetPlayer) _returnvalue)
      (Utilities|FlowControl|Sequence
        (:then_0
          (Timeline|VignetteTimeline ReverseFromEnd))
        (:then_1
          (Utilities|FlowControl|Delay 1.0)
          (Game|Player|SetViewTargetwithBlend _returnvalue (Game|GetPlayerCharacter 0) 1.0 "VTBlend_Linear" 0.0 false)
          (Utilities|FlowControl|Delay 0.2)
          (Class|UserTexturesTesterCharacter|SwitchonFlashlight (Variables|Default|GetPlayer)))))))

(fn ConstructionScript)

(fn GetHintText
  (return "Rest"))