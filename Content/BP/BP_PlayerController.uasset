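; Player controller that manages the game's HUD, menus and look sensitivity.
; On BeginPlay it creates the main HUD plus collapsed pause and texture-settings widgets, whose visibility functions also switch game pause, cursor, input mode and HUD.
; OpenSettings toggles a newly created SettingsUI, which returns to the pause menu when closed.
; A callback on the Input.Sensitivity console variable sets yaw scale and its negated pitch scale.
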(event Custom|CloseRequested
  (Widget|RemovefromParent (stale Custom|OpenSettings _returnvalue))
  (Variables|Default|SetbShowMouseCursor true)
  (Variables|Default|SetSettingsOpen false)
  (CallFunction|SetPauseMenuVisibility true))

(event Custom|SensitivityChanged
  (params (NewValue :type Float%20%28single-precision%29))
  (bind _output_get (Variables|Default|SetInputYawScale NewValue))
  (Variables|Default|SetInputPitchScale (* _output_get -1.0)))

(event Custom|OpenSettings
  (if (Variables|Default|GetSettingsOpen)
    (Widget|RemovefromParent (stale _returnvalue))
    (Variables|Default|SetbShowMouseCursor true)
    (Variables|Default|SetSettingsOpen false)
    (CallFunction|SetPauseMenuVisibility true)
    (else
      (bind _returnvalue (UserInterface|CreateWidget "/Game/UI/SettingsUI.SettingsUI_C"))
      (EventDispatchers|BindEventtoCloseRequested _returnvalue (delegate Custom|CloseRequested))
      (UserInterface|Viewport|AddtoViewport _returnvalue 0)
      (Variables|Default|SetbShowMouseCursor true)
      (Variables|Default|SetSettingsOpen true))))

(event EventTick
  (params (DeltaSeconds :type Float%20%28single-precision%29)))

(event EventBeginPlay
  (CallFunction|CreateWidgets)
  (Class|CVarChangeListenerManager|AddFloatCVarCallbackStatic "Input.Sensitivity" (delegate Custom|SensitivityChanged) true))

(fn ConstructionScript)

(fn CreateWidgets
  (bind _returnvalue (UserInterface|CreateWidget "/Game/Widgets/WB_PauseMenu.WB_PauseMenu_C"))
  (bind _output_get (Variables|Default|SetPauseWidget _returnvalue))
  (UserInterface|Viewport|AddtoViewport _output_get 0)
  (Widget|SetVisibility (Variables|Default|GetPauseWidget) "Collapsed")
  (bind _returnvalue_2 (UserInterface|CreateWidget "/Game/Widgets/WB_MainHud.WB_MainHUD_C" 0 (.AsBP%20Player%20Character (Utilities|Casting|CastToBP_PlayerCharacter (Pawn|GetControlledPawn))) self))
  (bind _output_get_2 (Variables|Default|SetMainHUD _returnvalue_2))
  (UserInterface|Viewport|AddtoViewport _output_get_2 0)
  (bind _returnvalue_3 (UserInterface|CreateWidget "/Game/ImportTexture/WB_TExtureSettings.WB_TextureSettings_C"))
  (bind _output_get_3 (Variables|Default|SetTextureSettings _returnvalue_3))
  (UserInterface|Viewport|AddtoViewport _output_get_3 0)
  (Widget|SetVisibility (Variables|Default|GetTextureSettings) "Collapsed"))

(fn SetPauseMenuVisibility
  (params (Visible? :type Boolean))
  (Game|SetGamePaused Visible?)
  (Widget|SetVisibility (Variables|Default|GetPauseWidget) (select Visible? "Visible" "Collapsed"))
  (bind _output_get (Variables|Default|SetbShowMouseCursor Visible?))
  (Widget|SetVisibility (Variables|Default|GetMainHUD) (select Visible? "Collapsed" "Visible"))
  (if _output_get
    (Input|SetInputModeUIOnly self (Variables|Default|GetPauseWidget) "DoNotLock")
    (Variables|Default|SetPauseOpen true)
    (else
      (Input|SetInputModeGameOnly self)
      (Variables|Default|SetPauseOpen false))))

(fn SetTextureMenuVisibility
  (params (Visible? :type Boolean))
  (Game|SetGamePaused Visible?)
  (Widget|SetVisibility (Variables|Default|GetTextureSettings) (select Visible? "Visible" "Collapsed"))
  (bind _output_get (Variables|Default|SetbShowMouseCursor Visible?))
  (Widget|SetVisibility (Variables|Default|GetMainHUD) (select Visible? "Collapsed" "Visible"))
  (if _output_get
    (Input|SetInputModeUIOnly self (Variables|Default|GetTextureSettings) "DoNotLock")
    (else
      (Input|SetInputModeGameOnly self))))