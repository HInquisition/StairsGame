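; BP_EnemyObserver is an enemy actor that always faces the player and kills them on contact.
; Each tick it rotates toward the player character and, while IsMoving is set, creeps toward them by a fixed per-frame step, not scaled by delta time, without sweeping.
; SetIsMoving toggles that movement, and overlapping the Box component calls PlayerDeath on BP_PlayerCharacter.
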(event OnComponentBeginOverlap(Box)
  (params (OverlappedComponent :type Primitive%20Component%20Object%20Reference) (OtherActor :type Actor%20Object%20Reference) (OtherComp :type Primitive%20Component%20Object%20Reference) (OtherBodyIndex :type Integer) (bFromSweep :type Boolean) (SweepResult :type Hit%20Result%20Structure%20%28by%20ref%29))
  (bind _asbp_player_character (Utilities|Casting|CastToBP_PlayerCharacter OtherActor))
  (Default|EventPlayerDeath _asbp_player_character))

(event EventBeginPlay)

(event Collision|EventActorBeginOverlap
  (params (OtherActor :type Actor%20Object%20Reference)))

(event EventTick
  (params (DeltaSeconds :type Float%20%28single-precision%29))
  (bind _returnvalue (Game|GetPlayerCharacter 0))
  (bind _returnvalue_2 (Transformation|GetActorLocation))
  (bind _returnvalue_3 (Transformation|GetActorLocation _returnvalue))
  (bind _returnvalue_4 (Math|Rotator|FindLookatRotation _returnvalue_2 _returnvalue_3))
  (Transformation|SetActorRotation _returnvalue_4)
  (if (Variables|Default|GetIsMoving?)
    (Transformation|SetActorLocation (+ (Transformation|GetActorLocation) (* (Math|Vector|GetForwardVector _returnvalue_4) 0.2)) false false)))

(fn ConstructionScript)

(fn SetIsMoving
  (params (Moving? :type Boolean))
  (Variables|Default|SetIsMoving? Moving?))