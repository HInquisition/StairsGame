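; BP_EnemyCharacter is a short-lived chaser enemy that constantly turns to face the player.
; Overlapping PlayerTrigger unpauses its audio and starts a self-repeating AIMoveTo toward the player, alongside a four-second delay that restores main-theme music and destroys the enemy.
; Overlapping KillTrigger fires the player's death event and also restores the music.
; The PawnSensing event is empty, and some debug and sound nodes are disconnected.
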(event OnComponentBeginOverlap(PlayerTrigger)
  (params (OverlappedComponent :type Primitive%20Component%20Object%20Reference) (OtherActor :type Actor%20Object%20Reference) (OtherComp :type Primitive%20Component%20Object%20Reference) (OtherBodyIndex :type Integer) (bFromSweep :type Boolean) (SweepResult :type Hit%20Result%20Structure%20%28by%20ref%29))
  (Utilities|Casting|CastToBP_PlayerCharacter OtherActor)
  (Class|AudioComponent|SetPaused (Variables|Default|GetAudio) false)
  (bind _movementresult (AI|AIMoveTo self "0, 0, 0" (Game|GetPlayerCharacter 0) 5.0 false :!label _label)
    (:then
      (Utilities|FlowControl|Delay 4.0)
      (bind _asbp_player_character (Utilities|Casting|CastToBP_PlayerCharacter (Game|GetPlayerCharacter 0)))
      (Default|SetMusicType _asbp_player_character "MainTheme")
      (Actor|DestroyActor))
    (:OnSuccess
      (Development|PrintString "Хряк на месте")
      (goto _label))
    (:OnFail
      (Development|PrintString (Utilities|String|EnumtoString _movementresult))
      (goto _label))))

(event OnComponentBeginOverlap(KillTrigger)
  (params (OverlappedComponent :type Primitive%20Component%20Object%20Reference) (OtherActor :type Actor%20Object%20Reference) (OtherComp :type Primitive%20Component%20Object%20Reference) (OtherBodyIndex :type Integer) (bFromSweep :type Boolean) (SweepResult :type Hit%20Result%20Structure%20%28by%20ref%29))
  (bind _asbp_player_character (Utilities|Casting|CastToBP_PlayerCharacter OtherActor))
  (Default|EventPlayerDeath _asbp_player_character)
  (bind _asbp_player_character_2 (Utilities|Casting|CastToBP_PlayerCharacter (Game|GetPlayerCharacter 0)))
  (Default|SetMusicType _asbp_player_character_2 "MainTheme"))

(event OnSeePawn(PawnSensing)
  (params (Pawn :type Pawn%20Object%20Reference)))

(event EventBeginPlay
  (Class|AudioComponent|SetPaused (Variables|Default|GetAudio) true))

(event EventTick
  (params (DeltaSeconds :type Float%20%28single-precision%29))
  (bind _returnvalue (Game|Player|GetPlayerPawn 0))
  (bind _returnvalue_2 (Transformation|GetActorLocation))
  (bind _returnvalue_3 (Transformation|GetActorLocation _returnvalue))
  (bind _returnvalue_4 (Math|Rotator|FindLookatRotation _returnvalue_2 _returnvalue_3))
  (Transformation|SetActorRotation (Math|Rotator|MakeRotator (.roll _returnvalue_4) 0.0 (.yaw _returnvalue_4))))

(fn ConstructionScript)