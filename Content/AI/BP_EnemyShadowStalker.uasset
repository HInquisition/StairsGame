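; Shadow stalker enemy that, when its reaction is triggered, runs at the player and vanishes after a few seconds.
; TriggerReaction calls the parent version, loops a zombie run animation and starts AIMoveTo on the first player character.
; A short Delay off the move's immediate output destroys the actor, while Success and Fail print a red debug result and re-issue the move.
; An unconnected sidestep SimpleMoveToLocation never runs.
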(event EventBeginPlay
  (|CallParentFunction))

(event Collision|EventActorBeginOverlap
  (params (OtherActor :type Actor%20Object%20Reference))
  (|CallParentFunction OtherActor) ; This node is disabled and will not be called.\nDrag off pins to build functionality.
)

(event EventTick
  (params (DeltaSeconds :type Float%20%28single-precision%29))
  (|CallParentFunction DeltaSeconds) ; This node is disabled and will not be called.\nDrag off pins to build functionality.
)

(event EventTriggerReaction
  (|CallParentFunction)
  (Components|Animation|PlayAnimation (Variables|Character|GetMesh) "/Game/Characters/MainEnemy/Zombie_Run_mixamo_com.Zombie_Run_mixamo_com" true)
  (bind _movementresult (AI|AIMoveTo self "0, 0, 0" (Game|GetPlayerCharacter 0) 5.0 false :!label _label)
    (:then
      (Utilities|FlowControl|Delay 4.0)
      (Actor|DestroyActor))
    (:OnSuccess
      (Development|PrintString (Utilities|String|EnumtoString _movementresult) true true "(R=1.000000,G=0.004170,B=0.000000,A=1.000000)")
      (goto _label))
    (:OnFail
      (Development|PrintString (Utilities|String|EnumtoString _movementresult) true true "(R=1.000000,G=0.004170,B=0.000000,A=1.000000)")
      (goto _label))))

(fn ConstructionScript
  (|CallParentFunction))