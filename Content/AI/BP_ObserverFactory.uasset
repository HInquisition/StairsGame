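; Factory actor that spawns BP_EnemyObserver enemies around the player and toggles their movement.
; SpawnObservers spawns ObserversNum observers at random offsets from the player, raised up to 1000 units; BeginPlay only delays and never calls it.
; NewFunction0 recurses until a sample is 5000+ units away, but returns a re-rolled point, so that distance is not guaranteed.
; SetObserversMoving passes a moving flag to every observer in the level.
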(event Custom|SpawnObservers
  (for _index (range 0 (- (Variables|Default|GetObserversNum) 1))
    (bind _returnvalue (CallFunction|NewFunction0))
    (Game|SpawnActorfromClass "/Game/AI/BP_EnemyObserver.BP_EnemyObserver_C" (Math|Transform|MakeTransform _returnvalue "0, 0, 0" (Math|Conversions|ToVector(Float) (Variables|Default|GetNewVar_0))) "Undefined" 0 0)))

(event EventBeginPlay
  (Utilities|FlowControl|Delay 0.2))

(event Collision|EventActorBeginOverlap
  (params (OtherActor :type Actor%20Object%20Reference)))

(event EventTick
  (params (DeltaSeconds :type Float%20%28single-precision%29)))

(fn ConstructionScript)

(fn NewFunction0
  (bind _returnvalue (Math|Random|RandomFloatinRange 0.0 1e+03))
  (bind _returnvalue_2 (Game|GetPlayerCharacter 0))
  (bind _newvar_1 (Variables|Default|GetNewVar_1))
  (bind _returnvalue_3 (Transformation|GetActorLocation _returnvalue_2))
  (bind _returnvalue_4 (* _newvar_1 -1.0))
  (bind _returnvalue_5 (Math|Random|RandomFloatinRange _returnvalue_4 _newvar_1))
  (bind _returnvalue_6 (Math|Random|RandomFloatinRange _returnvalue_4 _newvar_1))
  (bind _returnvalue_7 (Math|Vector|MakeVector _returnvalue_5 _returnvalue_6 _returnvalue))
  (bind _returnvalue_8 (+ _returnvalue_3 _returnvalue_7))
  (if (>= (Math|Vector|Distance(Vector) _returnvalue_8 _returnvalue_3) 5e+03)
    (return _returnvalue_8)
    (else
      (bind _returnvalue_9 (CallFunction|NewFunction0))
      (return _returnvalue_9))))

(fn SetObserversMoving
  (params (Moving? :type Boolean))
  (bind _outactors (Actor|GetAllActorsOfClass "/Game/AI/BP_EnemyObserver.BP_EnemyObserver_C"))
  (for _array_element _outactors
    (Default|SetIsMoving _array_element Moving?)))