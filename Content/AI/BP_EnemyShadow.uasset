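; BP_EnemyShadow is a shadow enemy that can kill the player on contact and is destroyed by light.
; InLight plays a monster sound and destroys the shadow after a brief delay.
; The Trigger overlap plays the same sound when the player enters and calls TriggerReaction, an empty event here.
; Player contact with Box1 prints debug text, then randomly either calls the player's death event, guarded by DoOnce, or destroys the shadow.
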(event OnComponentBeginOverlap(CapsuleComponent)
  (params (OverlappedComponent :type Primitive%20Component%20Object%20Reference) (OtherActor :type Actor%20Object%20Reference) (OtherComp :type Primitive%20Component%20Object%20Reference) (OtherBodyIndex :type Integer) (bFromSweep :type Boolean) (SweepResult :type Hit%20Result%20Structure%20%28by%20ref%29)))

(event OnComponentBeginOverlap(Box1)
  (params (OverlappedComponent :type Primitive%20Component%20Object%20Reference) (OtherActor :type Actor%20Object%20Reference) (OtherComp :type Primitive%20Component%20Object%20Reference) (OtherBodyIndex :type Integer) (bFromSweep :type Boolean) (SweepResult :type Hit%20Result%20Structure%20%28by%20ref%29))
  (bind _asbp_player_character (Utilities|Casting|CastToBP_PlayerCharacter OtherActor))
  (Development|PrintString "Боднул епта")
  (if (Math|Random|RandomBoolwithWeight 0.5)
    (Utilities|FlowControl|DoOnce false
      (:Completed
        (Default|EventPlayerDeath _asbp_player_character)))
    (else
      (Actor|DestroyActor))))

(event OnComponentBeginOverlap(Trigger)
  (params (OverlappedComponent :type Primitive%20Component%20Object%20Reference) (OtherActor :type Actor%20Object%20Reference) (OtherComp :type Primitive%20Component%20Object%20Reference) (OtherBodyIndex :type Integer) (bFromSweep :type Boolean) (SweepResult :type Hit%20Result%20Structure%20%28by%20ref%29))
  (Utilities|Casting|CastToBP_PlayerCharacter OtherActor)
  (Audio|PlaySound2D "/Game/Sounds/Monsters/Monster4.Monster4" 1.0 1.0 0.0 0 0)
  (CallFunction|TriggerReaction))

(event Custom|TriggerReaction)

(event EventBeginPlay)

(event Collision|EventActorBeginOverlap
  (params (OtherActor :type Actor%20Object%20Reference)))

(event EventTick
  (params (DeltaSeconds :type Float%20%28single-precision%29)))

(event EventInLight
  (Utilities|FlowControl|Delay 0.1)
  (Audio|PlaySound2D "/Game/Sounds/Monsters/Monster4.Monster4" 1.0 1.0 0.0 0 0)
  (Actor|DestroyActor))

(fn ConstructionScript)