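; BP_Hook is a monster hook attack that stretches an arm out to the player and drags them toward the actor.
; HookPlayer aborts if its visibility trace reports an initial overlap, otherwise starts the hook with monster and wind sounds.
; Tick poses PoseableMesh arm bones toward the player, then NewFunction0 teleports the player along a lerp.
; At 70% it calls CallPlayerNearEndOfHook, hides itself and stops the wind.
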(event Custom|HookPlayer
  (bind _returnvalue (Game|GetPlayerCharacter 0))
  (bind _outhit (Collision|LineTraceByChannel (Transformation|GetActorLocation) (Transformation|GetActorLocation _returnvalue) "TraceTypeQuery1" false (Utilities|Array|MakeArray _returnvalue) "None"))
  (if (.bInitialOverlap (Collision|BreakHitResult _outhit))
    (Development|PrintString "Cant hook")
    (else
      (Variables|Default|SetHooking? true)
      (Variables|Default|SetStart (Transformation|GetActorLocation (Game|GetPlayerCharacter 0)))
      (Default|PlayWindSound (Variables|Default|GetAs%20BP%20Player%20Character))
      (Audio|PlaySoundatLocation "/Game/Sounds/Monsters/Monster2.Monster2" (Transformation|GetActorLocation) "0, 0, 0" 1.0 1.0 0.0 0 0 0))))

(event EventBeginPlay
  (bind _asbp_player_character (Utilities|Casting|CastToBP_PlayerCharacter (Game|GetPlayerCharacter 0)))
  (Variables|Default|SetAs%20BP%20Player%20Character _asbp_player_character))

(event EventTick
  (params (DeltaSeconds :type Float%20%28single-precision%29))
  (bind _returnvalue (Game|GetPlayerCharacter 0))
  (bind _returnvalue_2 (Transformation|GetActorLocation))
  (bind _poseablemesh (Variables|Default|GetPoseableMesh))
  (bind _returnvalue_3 (Transformation|GetActorLocation _returnvalue))
  (bind _returnvalue_4 (Math|Rotator|FindLookatRotation _returnvalue_2 _returnvalue_3))
  (if (Variables|Default|GetHooking?)
    (if (> (Variables|Default|GetProgressToPlayer) 1.0)
      (CallFunction|NewFunction0 DeltaSeconds)
      (else
        (Variables|Default|SetProgressToPlayer (+ (* DeltaSeconds (Variables|Default|GetSpeed)) (Variables|Default|GetProgressToPlayer)))
        (Class|PoseableMeshComponent|SetBoneScalebyName _poseablemesh "LeftArm" "3.000000,3.000000,3.000000" "WorldSpace")
        (Components|PoseableMesh|SetBoneRotationbyName _poseablemesh "LeftArm" (Math|Rotator|MakeRotator (.roll _returnvalue_4) (.pitch _returnvalue_4) (+ (.yaw _returnvalue_4) 9e+01)) "WorldSpace")
        (Class|PoseableMeshComponent|SetBoneLocationbyName (Variables|Default|GetPoseableMesh) "LeftHand" (Math|Vector|Lerp(Vector) (+ (Transformation|GetActorLocation) "0, 0,100.000000") (Transformation|GetActorLocation (Game|GetPlayerCharacter 0)) (Variables|Default|GetProgressToPlayer)) "WorldSpace")
        (Class|PoseableMeshComponent|SetBoneLocationbyName (Variables|Default|GetPoseableMesh) "LeftArm" (Math|Vector|Lerp(Vector) (+ (Transformation|GetActorLocation) "0, 0,100.000000") (Transformation|GetActorLocation (Game|GetPlayerCharacter 0)) (Variables|Default|GetProgressToPlayer)) "WorldSpace")))))

(fn ConstructionScript)

(fn NewFunction0
  (params (A :type Float%20%28single-precision%29))
  (bind _returnvalue (Game|GetPlayerCharacter 0))
  (bind _returnvalue_2 (Transformation|GetActorLocation))
  (bind _returnvalue_3 (Game|GetPlayerCharacter 0))
  (bind _poseablemesh (Variables|Default|GetPoseableMesh))
  (bind _returnvalue_4 (Transformation|GetActorLocation _returnvalue))
  (bind _returnvalue_5 (Transformation|GetActorLocation _returnvalue_3))
  (bind _returnvalue_6 (Math|Rotator|FindLookatRotation _returnvalue_2 _returnvalue_4))
  (Variables|Default|SetProgress (+ (* A (Variables|Default|GetSpeed)) (Variables|Default|GetProgress)))
  (Class|PoseableMeshComponent|SetBoneScalebyName _poseablemesh "LeftArm" "3.000000,3.000000,3.000000" "WorldSpace")
  (Components|PoseableMesh|SetBoneRotationbyName _poseablemesh "LeftArm" (Math|Rotator|MakeRotator (.roll _returnvalue_6) (.pitch _returnvalue_6) (+ (.yaw _returnvalue_6) 9e+01)) "WorldSpace")
  (Class|PoseableMeshComponent|SetBoneLocationbyName (Variables|Default|GetPoseableMesh) "LeftHand" _returnvalue_5 "WorldSpace")
  (Class|PoseableMeshComponent|SetBoneLocationbyName (Variables|Default|GetPoseableMesh) "LeftArm" (Math|Vector|Lerp(Vector) (+ (Transformation|GetActorLocation) "0, 0,100.000000") _returnvalue_5 0.5) "WorldSpace")
  (if (< (Variables|Default|GetProgress) 0.7)
    (Transformation|SetActorLocation (Game|GetPlayerCharacter 0) (Math|Vector|Lerp(Vector) (Variables|Default|GetStart) (Transformation|GetActorLocation) (Variables|Default|GetProgress)) false true)
    (else
      (Default|CallPlayerNearEndOfHook)
      (Variables|Default|SetHooking? false)
      (Rendering|SetActorHiddenInGame true)
      (Default|StopWindSound (Variables|Default|GetAs%20BP%20Player%20Character)))))