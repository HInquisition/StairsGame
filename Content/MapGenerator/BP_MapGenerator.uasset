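; BP_MapGenerator manages player teleports between the main map and streamed Respawn, Exhausted Respawn and Observers levels, rather than generating terrain.
; BeginPlay creates the level instances far from the origin, with only Observers initially visible.
; Teleport functions toggle respawn-level streaming, move the player, switch music and, for some trips, adjust exhaustion.
; Observer trips save the return location, lazily spawn observers through BP_ObserverFactory, and have a timed variant.
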(event EventBeginPlay
  (|CallParentFunction)
  (bind _returnvalue (Class|LevelStreamingDynamic|LoadLevelInstance "PlayerRespawn" "100000.000000, 0,0.000000" "0, 0, 0"))
  (Variables|Default|SetRespawnLevel _returnvalue)
  (Variables|/Script/Engine.LevelStreaming|SetbShouldBeLoaded (Variables|Default|GetRespawnLevel) false)
  (Variables|/Script/Engine.LevelStreaming|SetbShouldBeVisible (Variables|Default|GetRespawnLevel) false)
  (bind _returnvalue_2 (Class|LevelStreamingDynamic|LoadLevelInstance "PlayerRespawnExhausted" "100000.000000,0.000000,0.000000" "0, 0, 0"))
  (Variables|Default|SetRespawnLevelExhausted _returnvalue_2)
  (Variables|/Script/Engine.LevelStreaming|SetbShouldBeLoaded (Variables|Default|GetRespawnLevelExhausted) false)
  (Variables|/Script/Engine.LevelStreaming|SetbShouldBeVisible (Variables|Default|GetRespawnLevelExhausted) false)
  (Variables|Default|SetPlayer%20Character (.AsBP%20Player%20Character (Utilities|Casting|CastToBP_PlayerCharacter (Game|GetPlayerCharacter 0))))
  (bind _returnvalue_3 (Class|LevelStreamingDynamic|LoadLevelInstance "Observers" "100000.000000,0.000000,-10000.000000" "0, 0, 0"))
  (Variables|Default|SetObserversLevel _returnvalue_3)
  (Variables|/Script/Engine.LevelStreaming|SetbShouldBeLoaded (Variables|Default|GetObserversLevel) true)
  (Variables|/Script/Engine.LevelStreaming|SetbShouldBeVisible (Variables|Default|GetObserversLevel) true))

(event Collision|EventActorBeginOverlap
  (params (OtherActor :type Actor%20Object%20Reference)))

(fn ConstructionScript)

(fn TptoRespawn
  (bind _respawnlevel (Variables|Default|GetRespawnLevel))
  (bind _player_character (Variables|Default|GetPlayer%20Character))
  (Variables|/Script/Engine.LevelStreaming|SetbShouldBeLoaded _respawnlevel true)
  (Variables|/Script/Engine.LevelStreaming|SetbShouldBeVisible _respawnlevel true)
  (Transformation|SetActorLocation (Game|GetPlayerCharacter 0) (Variables|Default|GetRespawnLocation) false false)
  (Default|SetMusicType _player_character "Peaceful")
  (Default|AddExhaustion _player_character -1e+01))

(fn TptoRespawnExhausted
  (bind _respawnlevelexhausted (Variables|Default|GetRespawnLevelExhausted))
  (Variables|/Script/Engine.LevelStreaming|SetbShouldBeLoaded _respawnlevelexhausted true)
  (Variables|/Script/Engine.LevelStreaming|SetbShouldBeVisible _respawnlevelexhausted true)
  (Transformation|SetActorLocation (Game|GetPlayerCharacter 0) (Variables|Default|GetRespawnLocationExhausted) false false)
  (Default|SetMusicType (Variables|Default|GetPlayer%20Character) "Danger"))

(fn TptoMap
  (bind _respawnlevel (Variables|Default|GetRespawnLevel))
  (bind _respawnlevelexhausted (Variables|Default|GetRespawnLevelExhausted))
  (Variables|/Script/Engine.LevelStreaming|SetbShouldBeLoaded _respawnlevelexhausted false)
  (Variables|/Script/Engine.LevelStreaming|SetbShouldBeVisible _respawnlevelexhausted false)
  (Variables|/Script/Engine.LevelStreaming|SetbShouldBeLoaded _respawnlevel false)
  (Variables|/Script/Engine.LevelStreaming|SetbShouldBeVisible _respawnlevel false)
  (Transformation|SetActorLocation (Game|GetPlayerCharacter 0) (Variables|Default|GetTpLocation) false false)
  (Default|SetMusicType (Variables|Default|GetPlayer%20Character) "MainTheme")
  (Default|AddExhaustion (Variables|Default|GetPlayer%20Character) 1e+01))

(fn TptoObservers
  (bind _observerslevel (Variables|Default|GetObserversLevel))
  (Variables|Default|SetBackFromObserversLocation (Transformation|GetActorLocation (Game|GetPlayerCharacter 0)))
  (Variables|/Game/BP/BP_PlayerCharacter.BP_PlayerCharacter_C|SetInObserversLevel? (Variables|Default|GetPlayer%20Character) true)
  (Variables|/Script/Engine.LevelStreaming|SetbShouldBeLoaded _observerslevel true)
  (Variables|/Script/Engine.LevelStreaming|SetbShouldBeVisible _observerslevel true)
  (Transformation|SetActorLocation (Game|GetPlayerCharacter 0) (Variables|Default|GetObserversLocation) false false)
  (if (Utilities|IsValid (Variables|Default|GetObserversManager))
    _
    (else
      (bind _outactors (Actor|GetAllActorsOfClass "/Game/AI/BP_ObserverFactory.BP_ObserverFactory_C"))
      (bind _output_get (Variables|Default|SetObserversManager (Utilities|Array|Get(acopy) _outactors)))
      (Default|SpawnObservers _output_get)))
  (Default|SetMusicType (Variables|Default|GetPlayer%20Character) "Danger")
  (Default|SetObserversMoving (Variables|Default|GetObserversManager) true))

(fn TpBackfromObservers
  (bind _observerslevel (Variables|Default|GetObserversLevel))
  (Transformation|SetActorLocation (Game|GetPlayerCharacter 0) (Variables|Default|GetBackFromObserversLocation) false false)
  (Default|SetMusicType (Variables|Default|GetPlayer%20Character) "MainTheme")
  (Default|SetObserversMoving (Variables|Default|GetObserversManager) true)
  (Variables|/Game/BP/BP_PlayerCharacter.BP_PlayerCharacter_C|SetInObserversLevel? (Variables|Default|GetPlayer%20Character) false)
  (Variables|/Script/Engine.LevelStreaming|SetbShouldBeLoaded _observerslevel true)
  (Variables|/Script/Engine.LevelStreaming|SetbShouldBeVisible _observerslevel true))

(fn TptoObserverTemporarily
  (params (BackDelay :type Float%20%28single-precision%29))
  (CallFunction|TptoObservers)
  (Utilities|Time|SetTimerbyEvent (EventDispatchers|CreateEvent :!event TpBackfromObservers) BackDelay))