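; A map generator floor tile that places a shadow screamer enemy in an unlit floor.
; On BeginPlay it sets the floor lighting to NotLighted before running the parent logic, then spawns BP_EnemyShadowScreamer at Scene0 and passes it the Box as its trigger.
; It then loads a NavMap level instance at SizeBox's location.
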(event EventBeginPlay
  (Variables|Default|SetFloorLightingType "NotLighted")
  (|CallParentFunction)
  (Game|SpawnActorfromClass "/Game/AI/BP_EnemyShadowScreamer.BP_EnemyShadowScreamer_C" (Math|Transform|MakeTransform (Transformation|GetWorldLocation (Variables|Default|GetScene_0)) "0, 0, 0" "1,1,1") "AdjustIfPossibleButAlwaysSpawn" 0 (Variables|Default|GetBox) 0)
  (bind _returnvalue (Class|LevelStreamingDynamic|LoadLevelInstance "NavMap" (Transformation|GetWorldLocation (Variables|Default|GetSizeBox)) "0, 0, 0"))
  (Variables|/Script/Engine.LevelStreaming|SetbShouldBeLoaded _returnvalue true))

(fn ConstructionScript
  (|CallParentFunction))