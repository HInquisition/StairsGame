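; BP_FloorShy is a map generator floor piece that spawns a shy enemy and shows a text hint for it.
; On BeginPlay, a 50/50 random roll picks between the passive and aggressive shy enemy variants and spawns it at the Scene0 component's location.
; The same roll sets the TextRender to "Look" for the passive variant or "Dont look" for the aggressive one.
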(event EventBeginPlay
  (|CallParentFunction)
  (bind _output_get (Variables|Default|SetRevers? (Math|Random|RandomBoolwithWeight 0.5)))
  (AI|SpawnAIFromClass (select _output_get "/Game/AI/BP_EnemyShyPassive.BP_EnemyShyPassive_C" "/Game/AI/BP_EnemyShyAggressive.BP_EnemyShyAggressive_C") 0 (Transformation|GetWorldLocation (Variables|Default|GetScene_0)) "0, 0, 0" false 0)
  (Rendering|Components|TextRender|SetText (Variables|Default|GetTextRender) (select (Variables|Default|GetRevers?) (Utilities|Text|MakeLiteralText "Look") (Utilities|Text|MakeLiteralText "Dont look"))))

(event Collision|EventActorBeginOverlap
  (params (OtherActor :type Actor%20Object%20Reference))
  (|CallParentFunction OtherActor) ; This node is disabled and will not be called.\nDrag off pins to build functionality.
)

(event EventTick
  (params (DeltaSeconds :type Float%20%28single-precision%29))
  (|CallParentFunction DeltaSeconds) ; This node is disabled and will not be called.\nDrag off pins to build functionality.
)

(fn ConstructionScript
  (|CallParentFunction))