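; BP_Floor is a map-generator floor actor that measures itself from its SizeBox, shows its floor number and sets up its lamps.
; On BeginPlay it takes the number from its Manager, writes it to a child BP_FloorDisplay, then runs InitLight.
; InitLight gathers child BP_Lamp actors and sets intensity and flicker by lighting type, randomised for partial and bad lighting.
; Entering the SizeBox sets the player's InLightFloor flag from that type.
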(event OnComponentBeginOverlap(SizeBox)
  (params (OverlappedComponent :type Primitive%20Component%20Object%20Reference) (OtherActor :type Actor%20Object%20Reference) (OtherComp :type Primitive%20Component%20Object%20Reference) (OtherBodyIndex :type Integer) (bFromSweep :type Boolean) (SweepResult :type Hit%20Result%20Structure%20%28by%20ref%29))
  (bind _floorlightingtype (Variables|Default|GetFloorLightingType))
  (bind _asbp_player_character (Utilities|Casting|CastToBP_PlayerCharacter OtherActor))
  (Variables|/Game/BP/BP_PlayerCharacter.BP_PlayerCharacter_C|SetInLightFloor? _asbp_player_character (Math|Boolean|ORBoolean (Utilities|Enum|Equal(Enum) _floorlightingtype "WellLighted") (Utilities|Enum|Equal(Enum) _floorlightingtype "PartiallyLighted") (Utilities|Enum|Equal(Enum) _floorlightingtype "BadLighted"))))

(event OnComponentEndOverlap(SizeBox)
  (params (OverlappedComponent :type Primitive%20Component%20Object%20Reference) (OtherActor :type Actor%20Object%20Reference) (OtherComp :type Primitive%20Component%20Object%20Reference) (OtherBodyIndex :type Integer))
  (bind _asbp_player_character (Utilities|Casting|CastToBP_PlayerCharacter OtherActor)))

(event Custom|InitializeFloor
  (Variables|Default|SetSize (* (Components|Box|GetScaledBoxExtent (Variables|Default|GetSizeBox)) 2))
  (Utilities|FlowControl|Delay 0.2)
  (bind _asbp_floor_display (Utilities|Casting|CastToBP_FloorDisplay (Variables|/Script/Engine.ChildActorComponent|GetChildActor (Variables|Default|GetDisplay))))
  (bind _output_get (Variables|Default|SetFloor%20Display _asbp_floor_display))
  (bind _manager (Variables|Default|GetManager)
    (:then
      (Default|SetText _output_get (Utilities|Text|ToText(Integer) (Variables|/Script/UserTexturesTester.FloorManager|GetFloorNumber _manager)))
      (Utilities|FlowControl|Delay 1.0)
      (CallFunction|InitLight))
    (:else
      (CallFunction|InitLight))))

(event EventBeginPlay
  (CallFunction|InitializeFloor))

(event Collision|EventActorBeginOverlap
  (params (OtherActor :type Actor%20Object%20Reference)))

(event EventTick
  (params (DeltaSeconds :type Float%20%28single-precision%29)))

(fn ConstructionScript)

(fn GetFloorSize
  (return (Variables|Default|GetSize)))

(fn InitLight
  (bind _lightintensitypercentage (Variables|Light|GetLightIntensityPercentage))
  (bind _lightdiversity (Variables|Light|GetLightDiversity))
  (bind _lightintensitypercentage_2 (Variables|Light|GetLightIntensityPercentage))
  (bind _lightdiversity_2 (Variables|Light|GetLightDiversity))
  (for _array_element (Actor|GetComponentsByClass "/Script/Engine.ChildActorComponent")
    (bind _asbp_lamp (Utilities|Casting|CastToBP_Lamp (Variables|/Script/Engine.ChildActorComponent|GetChildActor _array_element)))
    (Utilities|Array|Add (Variables|Light|GetLamps) _asbp_lamp))
  (Variables|Light|SetLightIntensityRuntime (Variables|Light|GetLightIntensity))
  (switch Utilities|FlowControl|Switch|SwitchonEFloorLightingType (Variables|Default|GetFloorLightingType)
    (:WellLighted
      (for _array_element_2 (Variables|Light|GetLamps) :!label _label
        (Default|SetLightParams _array_element_2 (Variables|Light|GetLightIntensityRuntime) (Variables|Light|GetLightColor) false)))
    (:PartiallyLighted
      (Variables|Light|SetLightIntensityRuntime (* (Variables|Light|GetLightIntensity) (Math|Float|Clamp(Float) (Math|Random|RandomFloatinRange (- _lightintensitypercentage_2 _lightdiversity_2) (+ _lightintensitypercentage_2 _lightdiversity_2)) 0.0 1.5)))
      (for _array_element_3 (Variables|Light|GetLamps)
        (Default|SetLightParams _array_element_3 (Math|Float|SelectFloat (Math|Float|SelectFloat (* (Variables|Light|GetLightIntensityRuntime) (+ (Variables|Light|GetLightDiversity) 1.0)) (* (Variables|Light|GetLightIntensityRuntime) (- 1.0 (Variables|Light|GetLightDiversity))) (Math|Random|RandomBoolwithWeight 0.5)) 0.0 (Math|Random|RandomBoolwithWeight 0.8)) (Variables|Light|GetLightColor) (Math|Random|RandomBoolwithWeight 0.5))))
    (:BadLighted
      (Variables|Light|SetLightIntensityRuntime (* (Variables|Light|GetLightIntensity) (Math|Float|Clamp(Float) (Math|Random|RandomFloatinRange (- _lightintensitypercentage _lightdiversity) (+ _lightintensitypercentage _lightdiversity)) 0.0 0.5)))
      (for _array_element_4 (Variables|Light|GetLamps)
        (Default|SetLightParams _array_element_4 (Math|Float|SelectFloat (Math|Float|SelectFloat (* (Variables|Light|GetLightIntensityRuntime) (+ (Variables|Light|GetLightDiversity) 1.0)) (* (Variables|Light|GetLightIntensityRuntime) (- 1.0 (Variables|Light|GetLightDiversity))) (Math|Random|RandomBoolwithWeight 0.2)) 0.0 (Math|Random|RandomBoolwithWeight 0.2)) (Variables|Light|GetLightColor) (Math|Random|RandomBoolwithWeight 0.5))))
    (:NotLighted
      (Variables|Light|SetLightIntensityRuntime 0.0)
      (goto _label))))