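; BP_FloorBlocked is a map floor piece with a wall, Plane7, that moves vertically when its child-actor button is activated.
; On BeginPlay it casts ChildActor60 to BP_Button and binds MoveWall to the button's activation event.
; MoveWall plays a quake sound and shakes the first player's camera while a timeline drives Plane7's relative Z.
; The shake stops immediately when the timeline finishes.
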(event Custom|MoveWall
  (bind _returnvalue (Game|GetPlayerController 0))
  (bind _plane7 (Variables|Default|GetPlane7))
  (bind _relativelocation (Variables|/Script/Engine.SceneComponent|GetRelativeLocation _plane7))
  (Audio|PlaySoundatLocation "/Game/Sounds/SC_Quake.SC_Quake" (Transformation|GetWorldLocation (Variables|Default|GetPlane7)) "0, 0, 0" 1.0 1.0 0.0 0 0 0)
  (Game|Feedback|ClientStartCameraShake _returnvalue "/Game/BP/CAmeraShake.CameraShake_C" 1.0 "CameraLocal" "0, 0, 0")
  (bind _newtrack_0 (Timeline|Timeline_0 Play)
    (:Update
      (Transformation|SetRelativeLocation _plane7 (Math|Vector|MakeVector (.x _relativelocation) (.y _relativelocation) _newtrack_0) false false))
    (:Finished
      (Game|Feedback|ClientStopCameraShake _returnvalue "/Game/BP/CAmeraShake.CameraShake_C" true))))

(event EventBeginPlay
  (|CallParentFunction)
  (bind _asbp_button (Utilities|Casting|CastToBP_Button (Variables|/Script/Engine.ChildActorComponent|GetChildActor (Variables|Default|GetChildActor6_0))))
  (EventDispatchers|BindEventtoButtonActivated _asbp_button (delegate Custom|MoveWall)))

(event Collision|EventActorBeginOverlap
  (params (OtherActor :type Actor%20Object%20Reference))
  (|CallParentFunction OtherActor) ; This node is disabled and will not be called.\nDrag off pins to build functionality.
)

(event EventTick
  (params (DeltaSeconds :type Float%20%28single-precision%29))
  (|CallParentFunction DeltaSeconds) ; This node is disabled and will not be called.\nDrag off pins to build functionality.
)

(fn ConstructionScript
  (|CallParentFunction))