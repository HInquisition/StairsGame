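; BP_FloorWithEnemy is a map generator floor piece that starts unlit and spawns an enemy.
; On BeginPlay it sets its lighting type to NotLighted, runs the parent logic, then spawns a BP_EnemyCharacter with SpawnAIFromClass at the Scene0 component.
; After a short delay it streams in a NavMap level instance at the SizeBox location, presumably to supply navigation for the AI.
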(event EventBeginPlay
  (Variables|Default|SetFloorLightingType "NotLighted")
  (|CallParentFunction)
  (AI|SpawnAIFromClass "/Game/AI/BP_EnemyCharacter.BP_EnemyCharacter_C" 0 (Transformation|GetWorldLocation (Variables|Default|GetScene_0)) "0, 0, 0" false 0)
  (Utilities|FlowControl|Delay 0.2)
  (bind _returnvalue (Class|LevelStreamingDynamic|LoadLevelInstance "NavMap" (Transformation|GetWorldLocation (Variables|Default|GetSizeBox)) "0, 0, 0"))
  (Variables|/Script/Engine.LevelStreaming|SetbShouldBeLoaded _returnvalue true))

(event Collision|EventActorBeginOverlap
  (params (OtherActor :type Actor%20Object%20Reference))
  (|CallParentFunction OtherActor) ; This node is disabled and will not be called.\nDrag off pins to build functionality.
)

(event EventTick
  (params (DeltaSeconds :type Float%20%28single-precision%29))
  (|CallParentFunction DeltaSeconds) ; This node is disabled and will not be called.\nDrag off pins to build functionality.
)

(fn ConstructionScript
  (|CallParentFunction))