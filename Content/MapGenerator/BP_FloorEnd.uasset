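; BP_FloorEnd is a trigger actor that plays the ending titles and returns the player to MainMap.
; When BP_PlayerCharacter overlaps its Box, input is disabled and a timeline drives the opacity of a WB_Dark overlay.
; When the timeline finishes, it collapses the overlay and plays WB_Titles.
; After a fixed delay for the titles, it sets OpenDoor on BP_GameInstance and opens MainMap.
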(event OnComponentBeginOverlap(Box)
  (params (OverlappedComponent :type Primitive%20Component%20Object%20Reference) (OtherActor :type Actor%20Object%20Reference) (OtherComp :type Primitive%20Component%20Object%20Reference) (OtherBodyIndex :type Integer) (bFromSweep :type Boolean) (SweepResult :type Hit%20Result%20Structure%20%28by%20ref%29))
  (Utilities|Casting|CastToBP_PlayerCharacter OtherActor)
  (bind _returnvalue (UserInterface|CreateWidget "/Game/Widgets/WB_Dark.WB_Dark_C" (Game|GetPlayerController 0)))
  (UserInterface|Viewport|AddtoViewport _returnvalue 0)
  (Input|DisableInput (Game|GetPlayerCharacter 0) (Game|GetPlayerController 0))
  (bind _newtrack_0 (Timeline|Timeline_0 Play)
    (:Update
      (Widget|SetRenderOpacity _returnvalue _newtrack_0))
    (:Finished
      (Widget|SetVisibility _returnvalue "Collapsed")
      (bind _returnvalue_2 (UserInterface|CreateWidget "/Game/Widgets/WB_Titles.WB_Titles_C" (Game|GetPlayerController 0)))
      (UserInterface|Viewport|AddtoViewport _returnvalue_2 0)
      (Default|PlayTitles _returnvalue_2)
      (Utilities|FlowControl|Delay 23.5)
      (bind _asbp_game_instance (Utilities|Casting|CastToBP_GameInstance (Game|GetGameInstance)))
      (Variables|/Game/BP/BP_GameInstance.BP_GameInstance_C|SetOpenDoor? _asbp_game_instance true)
      (Game|OpenLevel(byName) "MainMap"))))

(event EventBeginPlay
  (|CallParentFunction) ; This node is disabled and will not be called.\nDrag off pins to build functionality.
)

(event Collision|EventActorBeginOverlap
  (params (OtherActor :type Actor%20Object%20Reference))
  (|CallParentFunction OtherActor) ; This node is disabled and will not be called.\nDrag off pins to build functionality.
)

(event EventTick
  (params (DeltaSeconds :type Float%20%28single-precision%29))
  (|CallParentFunction DeltaSeconds) ; This node is disabled and will not be called.\nDrag off pins to build functionality.
)

(fn ConstructionScript
  (|CallParentFunction))