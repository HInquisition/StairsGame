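; Map generator floor piece where the player chooses one of three holes and dies on entering a wrong one.
; BeginPlay picks the right hole at random and shows its number on one of three randomly chosen text renders, hiding the others.
; Three box overlaps feed TriggerHandler, which kills the player character unless the box matches the right hole.
; BeginPlay also always spawns a shadow screamer enemy at Scene0, passing Box3 as its trigger.
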(event OnComponentBeginOverlap(Box)
  (params (OverlappedComponent :type Primitive%20Component%20Object%20Reference) (OtherActor :type Actor%20Object%20Reference) (OtherComp :type Primitive%20Component%20Object%20Reference) (OtherBodyIndex :type Integer) (bFromSweep :type Boolean) (SweepResult :type Hit%20Result%20Structure%20%28by%20ref%29))
  (CallFunction|TriggerHandler OtherActor))

(event OnComponentBeginOverlap(Box1)
  (params (OverlappedComponent :type Primitive%20Component%20Object%20Reference) (OtherActor :type Actor%20Object%20Reference) (OtherComp :type Primitive%20Component%20Object%20Reference) (OtherBodyIndex :type Integer) (bFromSweep :type Boolean) (SweepResult :type Hit%20Result%20Structure%20%28by%20ref%29))
  (CallFunction|TriggerHandler OtherActor 1))

(event OnComponentBeginOverlap(Box2)
  (params (OverlappedComponent :type Primitive%20Component%20Object%20Reference) (OtherActor :type Actor%20Object%20Reference) (OtherComp :type Primitive%20Component%20Object%20Reference) (OtherBodyIndex :type Integer) (bFromSweep :type Boolean) (SweepResult :type Hit%20Result%20Structure%20%28by%20ref%29))
  (CallFunction|TriggerHandler OtherActor 2))

(event EventBeginPlay
  (|CallParentFunction)
  (Rendering|SetVisibility (Variables|Default|GetTextRender3) false false)
  (Variables|Default|SetRightHole (Math|Random|RandomIntegerinRange 0 2))
  (bind _textrender (CallFunction|ChooseHoleTextRender (Math|Random|RandomIntegerinRange 0 2)))
  (Rendering|Components|TextRender|SetText _textrender (Utilities|Text|ToText(Integer) (+ (Variables|Default|GetRightHole) 1)))
  (Rendering|SetVisibility _textrender true false)
  (if (Math|Random|RandomBoolwithWeight 1.0)
    (Game|SpawnActorfromClass "/Game/AI/BP_EnemyShadowScreamer.BP_EnemyShadowScreamer_C" (Math|Transform|MakeTransform (Transformation|GetWorldLocation (Variables|Default|GetScene_0)) "0,90.000000, 0" "1,1,1") "Undefined" 0 (Variables|Default|GetBox3) 0)))

(fn ConstructionScript
  (|CallParentFunction))

(fn ChooseHoleTextRender
  (params (Hole :type Integer))
  (switch int Hole
    (:0
      (return (Variables|Default|GetTextRender)))
    (:1
      (return (Variables|Default|GetTextRender1)))
    (:2
      (return (Variables|Default|GetTextRender3)))))

(fn TriggerHandler
  (params (Object :type Actor%20Object%20Reference) (TriggerNum :type Integer))
  (bind _asbp_player_character (Utilities|Casting|CastToBP_PlayerCharacter Object))
  (if (not (== (Variables|Default|GetRightHole) TriggerNum))
    (Default|EventPlayerDeath _asbp_player_character)))