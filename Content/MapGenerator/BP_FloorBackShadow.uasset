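; Map generator floor actor, BP_FloorBackShadow, that adds danger music and a one-time enemy spawn.
; Shortly after BeginPlay it streams in a NavMap level instance at its SizeBox location.
; Player overlap with Box switches music to Danger, while overlap with Box1 spawns one BP_EnemyCharacter at Scene0.
; The music revert on leaving Box and the explosion sound are disconnected, so neither runs.
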(event OnComponentBeginOverlap(Box)
  (params (OverlappedComponent :type Primitive%20Component%20Object%20Reference) (OtherActor :type Actor%20Object%20Reference) (OtherComp :type Primitive%20Component%20Object%20Reference) (OtherBodyIndex :type Integer) (bFromSweep :type Boolean) (SweepResult :type Hit%20Result%20Structure%20%28by%20ref%29))
  (bind _asbp_player_character (Utilities|Casting|CastToBP_PlayerCharacter OtherActor))
  (Default|SetMusicType _asbp_player_character "Danger"))

(event OnComponentEndOverlap(Box)
  (params (OverlappedComponent :type Primitive%20Component%20Object%20Reference) (OtherActor :type Actor%20Object%20Reference) (OtherComp :type Primitive%20Component%20Object%20Reference) (OtherBodyIndex :type Integer))
  (bind _asbp_player_character (Utilities|Casting|CastToBP_PlayerCharacter OtherActor)))

(event OnComponentBeginOverlap(Box1)
  (params (OverlappedComponent :type Primitive%20Component%20Object%20Reference) (OtherActor :type Actor%20Object%20Reference) (OtherComp :type Primitive%20Component%20Object%20Reference) (OtherBodyIndex :type Integer) (bFromSweep :type Boolean) (SweepResult :type Hit%20Result%20Structure%20%28by%20ref%29))
  (Utilities|Casting|CastToBP_PlayerCharacter OtherActor)
  (Utilities|FlowControl|DoOnce false
    (:Completed
      (Game|SpawnActorfromClass "/Game/AI/BP_EnemyCharacter.BP_EnemyCharacter_C" (Math|Transform|MakeTransform (Transformation|GetWorldLocation (Variables|Default|GetScene_0)) "0, 0, 0" "1,1,1") "Undefined" 0 0))))

(event EventBeginPlay
  (|CallParentFunction)
  (Utilities|FlowControl|Delay 0.2)
  (bind _returnvalue (Class|LevelStreamingDynamic|LoadLevelInstance "NavMap" (Transformation|GetWorldLocation (Variables|Default|GetSizeBox)) "0.000000, 0, 0"))
  (Variables|/Script/Engine.LevelStreaming|SetbShouldBeLoaded _returnvalue true))

(event Collision|EventActorBeginOverlap
  (params (OtherActor :type Actor%20Object%20Reference))
  (|CallParentFunction OtherActor) ; This node is disabled and will not be called.\nDrag off pins to build functionality.
)

(event EventTick
  (params (DeltaSeconds :type Float%20%28single-precision%29))
  (|CallParentFunction DeltaSeconds) ; This node is disabled and will not be called.\nDrag off pins to build functionality.
)

(fn ConstructionScript
  (|CallParentFunction))