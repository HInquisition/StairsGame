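; BP_FloorWalls2 is a map generator piece, by its name a floor-and-walls variant, that can spawn a battery in the level.
; On BeginPlay it runs the parent logic, then on a 50% weighted random roll spawns a BP_Battery at the world transform of its Scene0 component.
; Overlap and Tick events are disabled, and the construction script only calls the parent.
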(event EventBeginPlay
  (|CallParentFunction)
  (if (Math|Random|RandomBoolwithWeight 0.5)
    (Game|SpawnActorfromClass "/Game/BP/BP_Battery.BP_Battery_C" (Transformation|GetWorldTransform (Variables|Default|GetScene_0)) "Undefined" 0 0)))

(event Collision|EventActorBeginOverlap
  (params (OtherActor :type Actor%20Object%20Reference))
  (|CallParentFunction OtherActor) ; This node is disabled and will not be called.\nDrag off pins to build functionality.
)

(event EventTick
  (params (DeltaSeconds :type Float%20%28single-precision%29))
  (|CallParentFunction DeltaSeconds) ; This node is disabled and will not be called.\nDrag off pins to build functionality.
)

(fn ConstructionScript
  (|CallParentFunction))