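; BP_FloorHook is a map-generator floor piece, marked well lighted, that carries the player along a hook and then relocates them.
; On BeginPlay it caches its child BP_Hook actor and registers a callback for when the player nears the hook's end.
; A player character overlapping the Box trigger starts the hook, and the callback teleports player 0 to the Scene0 component's location without sweeping.
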(event OnComponentBeginOverlap(Box)
  (params (OverlappedComponent :type Primitive%20Component%20Object%20Reference) (OtherActor :type Actor%20Object%20Reference) (OtherComp :type Primitive%20Component%20Object%20Reference) (OtherBodyIndex :type Integer) (bFromSweep :type Boolean) (SweepResult :type Hit%20Result%20Structure%20%28by%20ref%29))
  (Utilities|Casting|CastToBP_PlayerCharacter OtherActor)
  (Default|HookPlayer (Variables|Default|GetAs%20BP%20Hook)))

(event Custom|PlayerNearEndOfHook_Event_0
  (Transformation|SetActorLocation (Game|GetPlayerCharacter 0) (Transformation|GetWorldLocation (Variables|Default|GetScene_0)) false false))

(event EventBeginPlay
  (Variables|Default|SetFloorLightingType "WellLighted")
  (|CallParentFunction)
  (Variables|Default|SetAs%20BP%20Hook (.AsBP%20Hook (Utilities|Casting|CastToBP_Hook (Variables|/Script/Engine.ChildActorComponent|GetChildActor (Variables|Default|GetChildActor6_0)))))
  (EventDispatchers|AssignPlayerNearEndOfHook (Variables|Default|GetAs%20BP%20Hook) (delegate Custom|PlayerNearEndOfHook_Event_0)))

(event Collision|EventActorBeginOverlap
  (params (OtherActor :type Actor%20Object%20Reference))
  (|CallParentFunction OtherActor) ; This node is disabled and will not be called.\nDrag off pins to build functionality.
)

(event EventTick
  (params (DeltaSeconds :type Float%20%28single-precision%29))
  (|CallParentFunction DeltaSeconds) ; This node is disabled and will not be called.\nDrag off pins to build functionality.
)

(fn ConstructionScript
  (|CallParentFunction))