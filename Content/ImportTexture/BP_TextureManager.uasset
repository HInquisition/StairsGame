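; BP_TextureManager applies player-imported or default textures to the level's walls, floors and roofs, following the save game's settings.
; On BeginPlay it creates dynamic materials, then reloads from the save immediately and on a looping timer.
; Image files are imported at runtime into material parameters, then assigned by tag to BP_Floor components and StaticMeshActors.
; Roofs share the floor material, leaving RoofMat unused.
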(event Custom|CustomEvent_0
  (Utilities|Casting|CastToBP_PlayerController (Game|GetPlayerController 0))
  (CallFunction|LoadTexturesfromSave))

(event EventBeginPlay
  (bind _asbp_game_instance (Utilities|Casting|CastToBP_GameInstance (Game|GetGameInstance)))
  (Variables|Default|SetAs%20BP%20Game%20Instance _asbp_game_instance)
  (bind _returnvalue (Rendering|Material|CreateDynamicMaterialInstance "/Game/ImportTexture/M_LoadTextureWall.M_LoadTextureWall" "None" "None" :!class /Script/Engine.KismetMaterialLibrary))
  (Variables|Default|SetWallMat _returnvalue)
  (bind _returnvalue_2 (Rendering|Material|CreateDynamicMaterialInstance "/Game/ImportTexture/M_LoadTextureFloor.M_LoadTextureFloor" "None" "None" :!class /Script/Engine.KismetMaterialLibrary))
  (Variables|Default|SetFloorMat _returnvalue_2)
  (bind _returnvalue_3 (Rendering|Material|CreateDynamicMaterialInstance "/Game/ImportTexture/M_LoadTextureWall.M_LoadTextureWall" "None" "None" :!class /Script/Engine.KismetMaterialLibrary))
  (Variables|Default|SetRoofMat _returnvalue_3)
  (CallFunction|LoadTexturesfromSave)
  (Utilities|Time|SetTimerbyEvent (delegate Custom|CustomEvent_0) 4.0 true))

(fn ConstructionScript)

(fn SetMaterialbyTag
  (params (Tag :type Name) (Material :type Material%20Interface%20Object%20Reference))
  (Utilities|FlowControl|Sequence
    (:then_0
      (bind _outactors (Actor|GetAllActorsOfClass "/Game/MapGenerator/BP_Floor.BP_Floor_C"))
      (for _array_element _outactors
        (for _array_element_2 (Actor|GetComponentsbyTag _array_element "/Script/Engine.StaticMeshComponent" Tag)
          (Rendering|Material|SetMaterial _array_element_2 0 Material))))
    (:then_1
      (bind _outactors_2 (Actor|GetAllActorsOfClass "/Script/Engine.StaticMeshActor"))
      (bind _array_element_3 (Utilities|Array|ForEachLoopwithBreak _outactors_2)
        (:LoopBody
          (if (Actor|ActorHasTag _array_element_3 Tag)
            (Rendering|Material|SetMaterial (Variables|/Script/Engine.StaticMeshActor|GetStaticMeshComponent _array_element_3) 0 Material)))))))

(fn SetWallMaterialTexture
  (params (TexturePath :type String))
  (bind _output_get (Variables|Default|SetFilenameWall TexturePath))
  (bind _returnvalue (Class|KismetRenderingLibrary|ImportFileasTexture2D _output_get))
  (Rendering|Material|SetTextureParameterValue (Variables|Default|GetWallMat) "Texture" _returnvalue)
  (Variables|Default|SetUsingCustomWallTexture true))

(fn SetFloorMaterialTexture
  (params (TexturePath :type String))
  (bind _output_get (Variables|Default|SetFilenameFloor TexturePath))
  (bind _returnvalue (Class|KismetRenderingLibrary|ImportFileasTexture2D _output_get))
  (Rendering|Material|SetTextureParameterValue (Variables|Default|GetFloorMat) "Texture" _returnvalue)
  (Variables|Default|SetUsingCustomFloorTexture true))

(fn SetDefaultWallMaterial
  (Variables|Default|SetUsingCustomWallTexture false)
  (CallFunction|SetMaterialbyTag "Wall" "/Game/ImportTexture/M_Walls.M_Walls"))

(fn SetDefaultFloorMaterial
  (Variables|Default|SetUsingCustomFloorTexture false)
  (CallFunction|SetMaterialbyTag "Floor" "/Game/ImportTexture/M_Concrete_Poured2.M_Concrete_Poured2")
  (CallFunction|SetMaterialbyTag "Roof" "/Game/ImportTexture/M_Concrete_Poured2.M_Concrete_Poured2"))

(fn LoadTexturesfromSave
  (bind _savegame (CallFunction|GetSaveGame))
  (bind _floormat (Variables|Default|GetFloorMat))
  (Utilities|FlowControl|Sequence
    (:then_0
      (if (Variables|/Game/BP/BP_SaveGame.BP_SaveGame_C|GetUsingCustomFloorTexture _savegame)
        (bind _output_get (Variables|Default|SetFilenameFloor (Variables|/Game/BP/BP_SaveGame.BP_SaveGame_C|GetFilenameFloor _savegame)))
        (CallFunction|SetFloorMaterialTexture _output_get)
        (CallFunction|SetMaterialbyTag "Floor" _floormat)
        (CallFunction|SetMaterialbyTag "Roof" _floormat)
        (else
          (CallFunction|SetDefaultFloorMaterial))))
    (:then_1
      (if (Variables|/Game/BP/BP_SaveGame.BP_SaveGame_C|GetUsingCustomWallsTexture _savegame)
        (bind _output_get_2 (Variables|Default|SetFilenameWall (Variables|/Game/BP/BP_SaveGame.BP_SaveGame_C|GetFilenameWall _savegame)))
        (CallFunction|SetWallMaterialTexture _output_get_2)
        (CallFunction|SetMaterialbyTag "Wall" (Variables|Default|GetWallMat))
        (else
          (CallFunction|SetDefaultWallMaterial))))))